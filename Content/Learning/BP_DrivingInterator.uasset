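; Learning Agents interactor that lets an agent drive a sports car pawn around a track spline.
; Observations give the spline location and direction at the point nearest the car, plus its velocity, all relative to the car's transform.
; Actions are two floats: one sets steering, while the signed ThrottleBrake value applies throttle when positive and brake otherwise, zeroing the other input.
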(fn SpecifyAgentObservation
  (params (InObservationSchema :type Learning%20Agents%20Observation%20Schema%20Object%20Reference))
  (return (Class|LearningAgentsObservations|SpecifyStructObservation InObservationSchema (Utilities|Map|MakeMap "Track" (Class|LearningAgentsObservations|SpecifyStructObservation InObservationSchema (Utilities|Map|MakeMap "Location" (Class|LearningAgentsObservations|SpecifyLocationAlongSplineObservation InObservationSchema) "Direction" (Class|LearningAgentsObservations|SpecifyDirectionAlongSplineObservation InObservationSchema))) "Car" (Class|LearningAgentsObservations|SpecifyVelocityObservation InObservationSchema)))))

(fn GatherAgentObservation
  (params (InObservationObject :type Learning%20Agents%20Observation%20Object%20Object%20Reference) (AgentId :type Integer))
  (LocalVariables|SetObsActor (Class|LearningAgentsManagerListener|GetAgent AgentId "/Game/VehicleTemplate/Blueprints/SportsCar/SportsCar_Pawn.SportsCar_Pawn_C"))
  (return (Class|LearningAgentsObservations|MakeStructObservation InObservationObject (Utilities|Map|MakeMap "Track" (Class|LearningAgentsObservations|MakeStructObservation InObservationObject (Utilities|Map|MakeMap "Location" (Class|LearningAgentsObservations|MakeLocationAlongSplineObservation InObservationObject (Variables|Default|GetTrackSpline) (Class|SplineComponent|GetDistanceAlongSplineatLocation (Variables|Default|GetTrackSpline) (Transformation|GetActorLocation (LocalVariables|GetObsActor)) "World") (Transformation|GetActorTransform (LocalVariables|GetObsActor)) 1e+02 "LocationAlongSplineObservation" true 0) "Direction" (Class|LearningAgentsObservations|MakeDirectionAlongSplineObservation InObservationObject (Variables|Default|GetTrackSpline) (Class|SplineComponent|GetDistanceAlongSplineatLocation (Variables|Default|GetTrackSpline) (Transformation|GetActorLocation (LocalVariables|GetObsActor)) "World") (Transformation|GetActorTransform (LocalVariables|GetObsActor)) "DirectionAlongSplineObservation" true 0))) "Car" (Class|LearningAgentsObservations|MakeVelocityObservation InObservationObject (Transformation|GetVelocity (LocalVariables|GetObsActor)) (Transformation|GetActorTransform (LocalVariables|GetObsActor)) 2e+02 "VelocityObservation" true 0)))))

(fn SpecifyAgentAction
  (params (InActionSchema :type Learning%20Agents%20Action%20Schema%20Object%20Reference))
  (return (Class|LearningAgentsActions|SpecifyStructAction InActionSchema (Utilities|Map|MakeMap "Steering" (Class|LearningAgentsActions|SpecifyFloatAction InActionSchema "Steering") "ThrottleBrake" (Class|LearningAgentsActions|SpecifyFloatAction InActionSchema "ThrottleBrake")))))

(fn PerformAgentAction
  (params (InActionObject :type Learning%20Agents%20Action%20Object%20Object%20Reference) (InActionObjectElement :type Learning%20Agents%20Action%20Object%20Element%20Structure%20%28by%20ref%29) (AgentId :type Integer))
  (LocalVariables|SetActActor (Class|LearningAgentsManagerListener|GetAgent AgentId "/Game/VehicleTemplate/Blueprints/SportsCar/SportsCar_Pawn.SportsCar_Pawn_C"))
  (bind _outelements (Class|LearningAgentsActions|GetStructAction InActionObject InActionObjectElement))
  (Utilities|FlowControl|Sequence
    (:then_0
      (bind _outvalue (Class|LearningAgentsActions|GetFloatAction InActionObject (.Value (Utilities|Map|Find _outelements "Steering")) 1.0 "Steering" true 0))
      (Class|ChaosVehicleMovementComponent|SetSteeringInput (Variables|/Script/ChaosVehicles.WheeledVehiclePawn|GetVehicleMovementComponent (LocalVariables|GetActActor)) _outvalue))
    (:then_1
      (bind _outvalue_2 (Class|LearningAgentsActions|GetFloatAction InActionObject (.Value (Utilities|Map|Find _outelements "ThrottleBrake")) 1.0 "ThrottleBrake" true 0))
      (if (> _outvalue_2 0.0)
        (Class|ChaosVehicleMovementComponent|SetThrottleInput (Variables|/Script/ChaosVehicles.WheeledVehiclePawn|GetVehicleMovementComponent (LocalVariables|GetActActor)) _outvalue_2)
        (Class|ChaosVehicleMovementComponent|SetBrakeInput (Variables|/Script/ChaosVehicles.WheeledVehiclePawn|GetVehicleMovementComponent (LocalVariables|GetActActor)) 0.0)
        (else
          (Class|ChaosVehicleMovementComponent|SetBrakeInput (Variables|/Script/ChaosVehicles.WheeledVehiclePawn|GetVehicleMovementComponent (LocalVariables|GetActActor)) (- 0.0 _outvalue_2))
          (Class|ChaosVehicleMovementComponent|SetThrottleInput (Variables|/Script/ChaosVehicles.WheeledVehiclePawn|GetVehicleMovementComponent (LocalVariables|GetActActor)) 0.0))))))