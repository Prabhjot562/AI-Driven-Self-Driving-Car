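; Learning Agents reinforcement learning trainer that teaches SportsCar_Pawn agents to drive along a track spline.
; Reward combines velocity along the spline with a penalty for straying beyond a distance threshold from its closest point.
; Episode completion triggers on that same off-track threshold, and each reset moves the car to a random point on the spline.
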(fn GatherAgentReward
  (params (AgentId :type Integer))
  (LocalVariables|SetRewardActor (Class|LearningAgentsManagerListener|GetAgent AgentId "/Game/VehicleTemplate/Blueprints/SportsCar/SportsCar_Pawn.SportsCar_Pawn_C"))
  (return (+ (Class|LearningAgentsRewards|MakeRewardfromVelocityAlongSpline (Variables|Default|GetTrackSpline) (Transformation|GetActorLocation (LocalVariables|GetRewardActor)) (Transformation|GetVelocity (LocalVariables|GetRewardActor)) 1e+03 1.0 1e+01 "VelocityAlongSplineReward" true 0) (Class|LearningAgentsRewards|MakeRewardonLocationDifferenceAboveThreshold (Transformation|GetActorLocation (LocalVariables|GetRewardActor)) (Spline|FindLocationClosesttoWorldLocation (Variables|Default|GetTrackSpline) (Transformation|GetActorLocation (LocalVariables|GetRewardActor)) "World") 8e+02 -1e+01 "LocationDifferenceAboveThresholdReward" true 0))))

(fn GatherAgentCompletion
  (params (AgentId :type Integer))
  (bind _returnvalue (Class|LearningAgentsManagerListener|GetAgent AgentId "/Game/VehicleTemplate/Blueprints/SportsCar/SportsCar_Pawn.SportsCar_Pawn_C"))
  (bind _returnvalue_2 (Transformation|GetActorLocation _returnvalue))
  (return (Class|LearningAgentsCompletions|MakeCompletiononLocationDifferenceAboveThreshold (Spline|FindLocationClosesttoWorldLocation (Variables|Default|GetTrackSpline) _returnvalue_2 "World") _returnvalue_2 8e+02 "Termination" "LocationDifferenceAboveThresholdCompletion" false 0)))

(fn ResetAgentEpisode
  (params (AgentId :type Integer))
  (Default|ResettoRandomPointonSpline (Class|LearningAgentsManagerListener|GetAgent AgentId "/Game/VehicleTemplate/Blueprints/SportsCar/SportsCar_Pawn.SportsCar_Pawn_C") (Variables|Default|GetTrackSpline)))